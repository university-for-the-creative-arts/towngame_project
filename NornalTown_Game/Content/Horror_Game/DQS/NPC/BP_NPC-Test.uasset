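; Test NPC for the DQS dialogue system that starts a conversation, with a debug "Hello" print, whenever an actor overlaps it.
; Named DQS dialogue events route into a Gas Station Lines subgraph, which plays the matching voice line for each of the twelve gas station lines as 2D sound.
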(event Custom|StartConversation
  (Class|DQSDialogueParticipantComponent|StartDialogue (Variables|Default|GetDQSDialogueParticipant) self)
  (Development|PrintString "Hello"))

(event EventBeginPlay)

(event EventTick
  (params (DeltaSeconds :type Float%20%28single-precision%29)))

(event Collision|EventActorBeginOverlap
  (params (OtherActor :type Actor%20Object%20Reference))
  (CallFunction|StartConversation self))

(event EventDQSDialogueEvent
  (params (EventTag :type Gameplay%20Tag%20Structure) (EventName :type Name :default "None") (Context :type Object%20Object%20Reference))
  (switch name EventName
    (:Gas%20Station%20line%201
      (|GasStationLines :!label _label))
    (:Gas%20Station%20line%202
      (goto _label execute2))
    (:Gas%20Station%20line%203
      (goto _label execute3))
    (:Gas%20Station%20line%204
      (goto _label execute4))
    (:Gas%20Station%20line%205
      (goto _label execute5))
    (:Gas%20Station%20line%206
      (goto _label execute6))
    (:Gas%20Station%20line%207
      (goto _label execute7))
    (:Gas%20Station%20line%208
      (goto _label execute8))
    (:Gas%20Station%20line%209
      (goto _label execute9))
    (:Gas%20Station%20line%2010
      (goto _label execute10))
    (:Gas%20Station%20line%2011
      (goto _label execute11))
    (:Gas%20Station%20line%2012
      (goto _label execute12))))

(fn ConstructionScript)