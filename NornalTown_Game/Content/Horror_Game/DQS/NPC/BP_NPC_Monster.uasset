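; Monster NPC for a horror game that slowly turns to face the player and tracks damage until it is defeated.
; Tick interpolates its rotation toward the player character.
; AnyDamage lowers clamped health, broadcasts a health update, prints the value and sets a defeated flag at zero.
; BeginPlay creates a health bar widget bound to the monster, gated by the first-person character's GUNSALLOWED variable.
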(event Game|Damage|EventAnyDamage
  (params (Damage :type Float%20%28single-precision%29) (DamageType :type Damage%20Type%20Object%20Reference) (InstigatedBy :type Controller%20Object%20Reference) (DamageCauser :type Actor%20Object%20Reference))
  (Variables|Default|GetIS%20DEFEATED
    (:then)
    (:else
      (bind _output_get (Variables|Default|SetmonHP (Math|Float|Clamp(Float) (- (Variables|Default|GetmonHP) Damage) 0.0 7.0)))
      (Utilities|FlowControl|Sequence
        (:then_0
          (bind _newparam2 (CallFunction|NewFunction))
          (Variables|/Game/Horror_Game/DQS/UI/WBP_mon_HPbar.WBP_mon_HPbar_C|Setnext _newparam2 (+ (Variables|/Game/Horror_Game/DQS/UI/WBP_mon_HPbar.WBP_mon_HPbar_C|Getnext _newparam2) 1))
          (Default|CallEMonHealthUpdated _output_get (Variables|Default|GetmonMAXHP))
          (if (== _output_get 0.0)
            (Variables|Default|SetIS%20DEFEATED true)))
        (:then_1
          (Development|PrintString (Utilities|String|ToString(Float) _output_get)))))))

(event Collision|EventActorBeginOverlap
  (params (OtherActor :type Actor%20Object%20Reference)))

(event EventTick
  (params (DeltaSeconds :type Float%20%28single-precision%29))
  (Transformation|SetActorRotation (Math|Interpolation|RInterpTo (Transformation|GetActorRotation) (Math|Rotator|FindLookatRotation (Transformation|GetActorLocation) (Transformation|GetActorLocation (Game|GetPlayerCharacter 0))) DeltaSeconds 0.75)))

(event EventBeginPlay
  (bind _asbp_first_person_character (Utilities|Casting|CastToBP_FirstPersonCharacter (Game|GetPlayerCharacter 0)))
  (Variables|/Game/Horror_Game/Blueprints/BP_FirstPersonCharacter.BP_FirstPersonCharacter_C|GetGUNS%20ALLOWED _asbp_first_person_character
    (:then
      (bind _returnvalue (UserInterface|CreateWidget "/Game/Horror_Game/DQS/UI/WBP_mon_HPbar.WBP_mon_HPbar_C"))
      (UserInterface|Viewport|AddtoViewport _returnvalue 0)
      (Default|Happens _returnvalue self))
    (:else
      (Widget|RemovefromParent _returnvalue))))

(fn ConstructionScript)

(fn NewFunction
  (params (NewParam :type BP%20NPC%20Monster%20Object%20Reference))
  (return 0))