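; Horror game story sequencer that moves the player through a fixed chain of NPC encounters.
; Each Tick it reads OrderOfEvents from BP_FirstPersonGameMode and switches on it, with a DoOnce per stage.
; Stages spawn Samantha, James, then Nurse Mary at hardcoded transforms, each new stage destroying the previous NPC.
; Every stage after the first also plays a 2D sound, and the last only removes the nurse.
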(event Collision|EventActorBeginOverlap
  (params (OtherActor :type Actor%20Object%20Reference)))

(event EventTick
  (params (DeltaSeconds :type Float%20%28single-precision%29))
  (bind _asbp_first_person_game_mode (Utilities|Casting|CastToBP_FirstPersonGameMode (Game|GetGameMode)))
  (switch int (Variables|/Game/Horror_Game/Blueprints/BP_FirstPersonGameMode.BP_FirstPersonGameMode_C|Getorder%20of%20events _asbp_first_person_game_mode)
    (:0
      (Utilities|FlowControl|DoOnce false
        (:Completed
          (bind _returnvalue (|Samanthaspawn))
          (Variables|Default|SetGOD%20Woman%20Return _returnvalue))))
    (:1
      (Utilities|FlowControl|DoOnce false
        (:Completed
          (Audio|PlaySound2D "/Game/Horror_Game/Audio/Other/VA_lines/MercenaryVirgil/1892WasAWhileAgo.1892WasAWhileAgo" 1.0 1.0 0.0 "/Game/Horror_Game/Audio/Other/VA_lines/SC_VA.SC_VA" 0)
          (Actor|DestroyActor (Variables|Default|GetGOD%20Woman%20Return))
          (bind _returnvalue_2 (|JamesSpawn))
          (Variables|Default|SetGOD%20Man%20Return _returnvalue_2))))
    (:2
      (Utilities|FlowControl|DoOnce false
        (:Completed
          (Audio|PlaySound2D "/Game/Horror_Game/Audio/Other/VA_lines/MercenaryVirgil/LifestyleChanges.LifestyleChanges" 1.0 1.0 0.0 "/Game/Horror_Game/Audio/Other/VA_lines/SC_VA.SC_VA" 0)
          (Actor|DestroyActor (Variables|Default|GetGOD%20Man%20Return))
          (bind _returnvalue_3 (|NurseSpawn))
          (Variables|Default|SetWeird%20Nurse%20Return _returnvalue_3))))
    (:3
      (Utilities|FlowControl|DoOnce false
        (:Completed
          (Audio|PlaySound2D "/Game/Horror_Game/Audio/Other/VA_lines/MercenaryVirgil/CreatureTheChurch.CreatureTheChurch" 1.0 1.0 0.0 "/Game/Horror_Game/Audio/Other/VA_lines/SC_VA.SC_VA" 0)
          (Actor|DestroyActor (Variables|Default|GetWeird%20Nurse%20Return)))))))

(fn ConstructionScript)