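; BP_ChurchDoors is a horror-game actor that swings a pair of church doors when the game's event sequence reaches step 4.
; Tick polls OrderOfEvents on BP_FirstPersonGameMode, and a DoOnce limits the trigger to a single firing.
; Two timelines, started in sequence, drive the relative yaw of the left and right doors through Lerps whose zero Alpha passes the track value straight through.
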(event EventTick
  (params (DeltaSeconds :type Float%20%28single-precision%29))
  (bind _asbp_first_person_game_mode (Utilities|Casting|CastToBP_FirstPersonGameMode (Game|GetGameMode)))
  (if (== (Variables|/Game/Horror_Game/Blueprints/BP_FirstPersonGameMode.BP_FirstPersonGameMode_C|Getorder%20of%20events _asbp_first_person_game_mode) 4)
    (Utilities|FlowControl|DoOnce false
      (:Completed
        (Utilities|FlowControl|Sequence
          (:then_0
            (bind _left (Timeline|Doorleft Play)
              (:Update
                (Transformation|SetRelativeRotation (Variables|Default|Getdoor%20left) (Math|Rotator|MakeRotator 0.0 0.0 (Math|Float|Lerp _left 0.0 0.0)) false false))))
          (:then_1
            (bind _right (Timeline|DoorRight Play)
              (:Update
                (Transformation|SetRelativeRotation (Variables|Default|Getdoor%20right) (Math|Rotator|MakeRotator 0.0 0.0 (Math|Float|Lerp _right 0.0 0.0)) false false)))))))))

(fn ConstructionScript)