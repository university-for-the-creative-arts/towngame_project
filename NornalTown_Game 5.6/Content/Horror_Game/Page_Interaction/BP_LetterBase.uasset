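; BP_LetterBase is an interactable letter for the horror game that shows its text on screen.
; Interact creates a WB_Letter widget from the Text variable on first use, caches it, then toggles it in and out of the viewport.
; When BP_FirstPersonCharacter stops overlapping the LetterOne component, the widget is removed from the screen.
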(event OnComponentEndOverlap(LetterOne)
  (params (OverlappedComponent :type Primitive%20Component%20Object%20Reference) (OtherActor :type Actor%20Object%20Reference) (OtherComp :type Primitive%20Component%20Object%20Reference) (OtherBodyIndex :type Integer))
  (if (.bSuccess (Utilities|Casting|CastToBP_FirstPersonCharacter OtherActor))
    (bind _letterwidget (Variables|Default|GetLetterWidget)
      (:then
        (Widget|RemovefromParent _letterwidget))
      (:else))))

(event EventInteract
  (Variables|Default|GetLetterWidget
    (:then
      _)
    (:else
      (bind _returnvalue (UserInterface|CreateWidget "/Game/Horror_Game/Page_Interaction/WB_Letter.WB_Letter_C" 0 (Utilities|Text|ToText(String) (Variables|Default|GetText))))
      (Variables|Default|SetLetterWidget _returnvalue)))
  (if (UserInterface|Viewport|IsinViewport (Variables|Default|GetLetterWidget))
    (Widget|RemovefromParent (Variables|Default|GetLetterWidget))
    (else
      (UserInterface|Viewport|AddtoViewport (Variables|Default|GetLetterWidget) 0))))

(fn ConstructionScript)