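; BP_monster is a monster NPC for the horror game that takes damage and reports progress to BP_FirstPersonGameMode.
; While not defeated, each hit lowers its clamped health and increments the game mode's NEXT counter.
; At zero health it sets ISDEFEATED, then runs a short delay with nothing after it.
; Separately, pressing E sets the game mode's OrderOfEvents to a fixed step, with no proximity or state check.
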(event Game|Damage|EventAnyDamage
  (params (Damage :type Float%20%28single-precision%29) (DamageType :type Damage%20Type%20Object%20Reference) (InstigatedBy :type Controller%20Object%20Reference) (DamageCauser :type Actor%20Object%20Reference))
  (Variables|Default|GetIS%20DEFEATED
    (:then)
    (:else
      (bind _output_get (Variables|Default|SetmonHP (Math|Float|Clamp(Float) (- (Variables|Default|GetmonHP) Damage) 0.0 7.0)))
      (bind _asbp_first_person_game_mode (Utilities|Casting|CastToBP_FirstPersonGameMode (Game|GetGameMode)))
      (Variables|/Game/Horror_Game/Blueprints/BP_FirstPersonGameMode.BP_FirstPersonGameMode_C|SetNEXT _asbp_first_person_game_mode (+ (Variables|/Game/Horror_Game/Blueprints/BP_FirstPersonGameMode.BP_FirstPersonGameMode_C|GetNEXT _asbp_first_person_game_mode) 1))
      (if (== _output_get 0.0)
        (Variables|Default|SetIS%20DEFEATED true)
        (Utilities|FlowControl|Delay 0.5)))))

(event Collision|EventActorBeginOverlap
  (params (OtherActor :type Actor%20Object%20Reference)))

(event Input|KeyboardEvents|DebugKeyE
  (params (Key :type Key%20Structure :default "None") (ActionValue :type Input%20Action%20Value%20Structure)))

(event Input|KeyboardEvents|E
  (params (Key :type Key%20Structure :default "None"))
  (:Pressed
    (bind _asbp_first_person_game_mode (Utilities|Casting|CastToBP_FirstPersonGameMode (Game|GetGameMode)))
    (Variables|/Game/Horror_Game/Blueprints/BP_FirstPersonGameMode.BP_FirstPersonGameMode_C|Setorder%20of%20events _asbp_first_person_game_mode 5)))

(fn ConstructionScript)