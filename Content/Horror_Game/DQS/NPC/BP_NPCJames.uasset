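; BP_NPCJames is an NPC actor that starts a DQS dialogue when any actor overlaps it and prints a debug "Hello".
; DQS dialogue events named for eight "Town P2" lines are matched and routed into a collapsed "town P1 Lines" graph.
; That graph plays the matching voice line as a 2D sound, and also holds four unconnected sound calls that never run.
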(event Custom|StartConversation
  (Class|DQSDialogueParticipantComponent|StartDialogue (Variables|Default|GetDQSDialogueParticipant) self)
  (Development|PrintString "Hello"))

(event EventBeginPlay)

(event EventTick
  (params (DeltaSeconds :type Float%20%28single-precision%29)))

(event Collision|EventActorBeginOverlap
  (params (OtherActor :type Actor%20Object%20Reference))
  (CallFunction|StartConversation self))

(event EventDQSDialogueEvent
  (params (EventTag :type Gameplay%20Tag%20Structure) (EventName :type Name :default "None") (Context :type Object%20Object%20Reference))
  (switch name EventName
    (:Town%20P2%20line%201
      (|townP1Lines :!label _label))
    (:Town%20P2%20line%202
      (goto _label execute2))
    (:Town%20P2%20line%203
      (goto _label execute3))
    (:Town%20P2%20%20line%204
      (goto _label execute4))
    (:Town%20P2%20line%205
      (goto _label execute5))
    (:Town%20P2%20line%206
      (goto _label execute6))
    (:Town%20P2%20line%207
      (goto _label execute7))
    (:Town%20P2%20line%208
      (goto _label execute8))))

(fn ConstructionScript)